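; BP_Overheadlight_01 is an overhead light for the subway train, with a point light and a spot light driven by custom events.
; SetIntensity passes the value straight to the point light and gives the spot light only the whole-number quotient of a fixed division.
; Despite its name, SetRandomColor applies a fixed blue tint to the point light; its random nodes and spot-light color call are disconnected.
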(event `SetIntensity`
  (params (Intensity :type "Float (double-precision)"))
  (`LightComponent.SetIntensity` (`self.PointLight`) Intensity)
  (`LightComponent.SetIntensity` (`self.SpotLight`) (`KismetMathLibrary.Conv_IntToDouble` (`.ReturnValue` (`KismetMathLibrary.FMod` Intensity 2000.0)))))

(event `SetRandomColor`
  (`LightComponent.SetLightColor` (`self.PointLight`) (make `LinearColor` 0.2 0.0 1.0 1.0) true))

(fn `UserConstructionScript`)