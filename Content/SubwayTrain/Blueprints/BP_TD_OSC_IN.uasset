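; Receives OSC bundles to drive the intensity of the subway scene's overhead lights.
; On BeginPlay it starts a listening OSC server and randomizes the color of all BPOverheadLight actors.
; The first message in each bundle is matched on its address, and its first float sets one light's intensity through hard-coded, out-of-order array indices.
; The sixth channel also switches a second light to zero.
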(event `self.ReceiveBeginPlay`
  ;[1 1 1] Binding to Any Message
  (bind _returnvalue (`OSCManager.CreateOSCServer` (`self.Receive IPAddress`) (`self.Port`) false true "UE_OSC" null))
  (bind _output_get (set `self.TD_OSC_Server` _returnvalue))
  (add `OSCServer.OnOscBundleReceived` _output_get (delegate `OnBundleReceived`))
  (bind _outactors (`GameplayStatics.GetAllActorsOfClass` (`self.BP_Overhead_Light`)))
  (`/Game/SubwayTrain/Blueprints/BP_Overheadlight_01.SetRandomColor` _outactors))

(event `OnMsgReceived`
  (params (Message :type "OSCMessage Structure (by ref)") (IPAddress :type String) (Port :type Integer))
  ;[1 1 1] Binding to Any Message
)

(event `OnBundleReceived`
  (params (Bundle :type "OSCBundle Structure (by ref)") (IPAddress :type String) (Port :type Integer))
  ;[1 1 1] Binding to Any Message
  (bind (_bsucceeded _returnvalue) (`OSCManager.GetMessageFromBundle` Bundle))
  (bind _returnvalue_2 (`OSCManager.GetOSCMessageAddress` _returnvalue))
  (bind _returnvalue_3 (`OSCManager.GetOSCAddressFullPath` _returnvalue_2))
  (switch `string` _returnvalue_3
    (:`/intensity1`
      (bind _values (`OSCManager.GetAllFloats` _returnvalue))
      (`/Game/SubwayTrain/Blueprints/BP_Overheadlight_01.SetIntensity` (`|GetArrayItem` (stale `self.ReceiveBeginPlay` _outactors)) (`|GetArrayItem` _values)))
    (:`/intensity2`
      (bind _values_2 (`OSCManager.GetAllFloats` _returnvalue))
      (`/Game/SubwayTrain/Blueprints/BP_Overheadlight_01.SetIntensity` (`|GetArrayItem` (stale `self.ReceiveBeginPlay` _outactors) 5) (`|GetArrayItem` _values_2)))
    (:`/intensity3`
      (bind _values_3 (`OSCManager.GetAllFloats` _returnvalue))
      (`/Game/SubwayTrain/Blueprints/BP_Overheadlight_01.SetIntensity` (`|GetArrayItem` (stale `self.ReceiveBeginPlay` _outactors) 6) (`|GetArrayItem` _values_3)))
    (:`/intensity4`
      (bind _values_4 (`OSCManager.GetAllFloats` _returnvalue))
      (`/Game/SubwayTrain/Blueprints/BP_Overheadlight_01.SetIntensity` (`|GetArrayItem` (stale `self.ReceiveBeginPlay` _outactors) 7) (`|GetArrayItem` _values_4)))
    (:`/intensity5`
      (bind _values_5 (`OSCManager.GetAllFloats` _returnvalue))
      (`/Game/SubwayTrain/Blueprints/BP_Overheadlight_01.SetIntensity` (`|GetArrayItem` (stale `self.ReceiveBeginPlay` _outactors) 2) (`|GetArrayItem` _values_5)))
    (:`/intensity6`
      (bind _values_6 (`OSCManager.GetAllFloats` _returnvalue))
      (`/Game/SubwayTrain/Blueprints/BP_Overheadlight_01.SetIntensity` (`|GetArrayItem` (stale `self.ReceiveBeginPlay` _outactors) 4) (`|GetArrayItem` _values_6))
      (bind _values_7 (`OSCManager.GetAllFloats` _returnvalue))
      (`/Game/SubwayTrain/Blueprints/BP_Overheadlight_01.SetIntensity` (`|GetArrayItem` (stale `self.ReceiveBeginPlay` _outactors) 9) 0.0))
    (:`/intensity7`
      (bind _values_8 (`OSCManager.GetAllFloats` _returnvalue))
      (`/Game/SubwayTrain/Blueprints/BP_Overheadlight_01.SetIntensity` (`|GetArrayItem` (stale `self.ReceiveBeginPlay` _outactors) 1) (`|GetArrayItem` _values_8)))
    (:`/intensity8`
      (bind _values_9 (`OSCManager.GetAllFloats` _returnvalue))
      (`/Game/SubwayTrain/Blueprints/BP_Overheadlight_01.SetIntensity` (`|GetArrayItem` (stale `self.ReceiveBeginPlay` _outactors) 10) (`|GetArrayItem` _values_9)))
    (:`/intensity9`
      (bind _values_10 (`OSCManager.GetAllFloats` _returnvalue))
      (`/Game/SubwayTrain/Blueprints/BP_Overheadlight_01.SetIntensity` (`|GetArrayItem` (stale `self.ReceiveBeginPlay` _outactors) 3) (`|GetArrayItem` _values_10)))
    (:`/intensity10`
      (bind _values_11 (`OSCManager.GetAllFloats` _returnvalue))
      (`/Game/SubwayTrain/Blueprints/BP_Overheadlight_01.SetIntensity` (`|GetArrayItem` (stale `self.ReceiveBeginPlay` _outactors) 8) (`|GetArrayItem` _values_11)))))

(fn `UserConstructionScript`)